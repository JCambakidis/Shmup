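; Boss enemy for a shoot 'em up that fires bullet-hell patterns and, on death, spawns an explosion and calls EndGame on the player.
; Shoot re-arms itself by timer and, once in place, picks one of three patterns by remaining thirds of starting life.
; Patterns chain or overlap HellLoopShoot macros, which spawn projectiles across an arc through a delayed loop.
; Two timelines offset Y and Z around TargetLocation when ActiononStop fires.
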(event EventBeginPlay
  (|CallParentFunction)
  (Utilities|FlowControl|Delay 0.2)
  (Variables|Default|SetCan%20Shoot true)
  (CallFunction|Shoot)
  (Variables|Default|SetInit%20Life_0 (Variables|Default|GetLife)))

(event Collision|EventActorBeginOverlap
  (params (OtherActor :type Actor%20Object%20Reference))
  (|CallParentFunction OtherActor) ; This node is disabled and will not be called.\nDrag off pins to build functionality.
)

(event EventTick
  (params (DeltaSeconds :type Float%20%28single-precision%29))
  (|CallParentFunction DeltaSeconds))

(event EventShoot
  (bind _life (Variables|Default|GetLife))
  (bind _init_life_0 (Variables|Default|GetInit%20Life_0))
  (bind _returnvalue (/ _init_life_0 3))
  (if (and (Variables|Default|GetCan%20Shoot) (Variables|Default|GetIn%20place))
    (if (> _life (* _returnvalue 2))
      (Utilities|FlowControl|Sequence
        (:then_0
          (Utilities|HellLoopShoot "/Game/Shmup/Blueprints/Projectiles/Enemy_simpleshoot_BP.Enemy_simpleshoot_BP_C" 0.05 (Transformation|GetActorLocation) "3.000000,3.000000,3.000000" 30 0 360
            (:Complete
              (Utilities|HellLoopShoot "/Game/Shmup/Blueprints/Projectiles/Enemy_simpleshoot_BP.Enemy_simpleshoot_BP_C" 0.05 (Transformation|GetActorLocation) "3.000000,3.000000,3.000000" 30 360
                (:Complete
                  (Utilities|Time|SetTimerbyEvent (delegate EventShoot) (Variables|Default|GetShoot%20speed) :!label _label))))))
        (:then_1
          (Utilities|HellLoopShoot "/Game/Shmup/Blueprints/Projectiles/Enemy_simpleshoot_BP.Enemy_simpleshoot_BP_C" 0.0 (Transformation|GetActorLocation) "3.000000,3.000000,3.000000" 30 0 360 :!label _label_2
            (:Complete
              (Utilities|HellLoopShoot "/Game/Shmup/Blueprints/Projectiles/Enemy_simpleshoot_BP.Enemy_simpleshoot_BP_C" 0.0 (Transformation|GetActorLocation) "3.000000,3.000000,3.000000" 30 0 360)))))
      (elif (> _life _returnvalue)
        (Utilities|FlowControl|Sequence
          (:then_0
            (Utilities|HellLoopShoot "/Game/Shmup/Blueprints/Projectiles/Enemy_simpleshoot_BP.Enemy_simpleshoot_BP_C" 0.04 (Transformation|GetActorLocation) "3.000000,3.000000,3.000000" 30 0 360
              (:Complete
                (goto _label))))
          (:then_1
            (Utilities|HellLoopShoot "/Game/Shmup/Blueprints/Projectiles/Enemy_simpleshoot_BP.Enemy_simpleshoot_BP_C" 0.04 (Transformation|GetActorLocation) "3.000000,3.000000,3.000000" 30 360))
          (:then_2
            (goto _label_2)))
        (else
          (Utilities|HellLoopShoot "/Game/Shmup/Blueprints/Projectiles/Enemy_simpleshoot_BP.Enemy_simpleshoot_BP_C" 0.0 (Transformation|GetActorLocation) "3.000000,3.000000,3.000000" 30 0 360
            (:Complete
              (Utilities|HellLoopShoot "/Game/Shmup/Blueprints/Projectiles/Enemy_simpleshoot_BP.Enemy_simpleshoot_BP_C" 0.02 (Transformation|GetActorLocation) "3.000000,3.000000,3.000000" 30 0 -90
                (:Complete
                  (Utilities|HellLoopShoot "/Game/Shmup/Blueprints/Projectiles/Enemy_simpleshoot_BP.Enemy_simpleshoot_BP_C" 0.02 (Transformation|GetActorLocation) "3.000000,3.000000,3.000000" 30 -180 -90
                    (:Complete
                      (Utilities|FlowControl|Sequence
                        (:then_0
                          (Utilities|HellLoopShoot "/Game/Shmup/Blueprints/Projectiles/Enemy_simpleshoot_BP.Enemy_simpleshoot_BP_C" 0.01 (Transformation|GetActorLocation) "3.000000,3.000000,3.000000" 30 0 360
                            (:Complete
                              (goto _label))))
                        (:then_1
                          (Utilities|HellLoopShoot "/Game/Shmup/Blueprints/Projectiles/Enemy_simpleshoot_BP.Enemy_simpleshoot_BP_C" 0.01 (Transformation|GetActorLocation) "3.000000,3.000000,3.000000" 30 360))))))))))))
    (else
      (goto _label))))

(event EventActiononStop
  (bind _returnvalue (Transformation|GetActorLocation))
  (bind _returnvalue_2 (Transformation|GetActorLocation))
  (bind _target_location (Variables|Default|GetTarget%20Location))
  (Utilities|FlowControl|Sequence
    (:then_0
      (bind _newtrack_1 (Timeline|Movement PlayFromStart)
        (:Update
          (Transformation|SetActorLocation (Math|Vector|MakeVector (.x _returnvalue_2) (.y _returnvalue_2) (+ (.z _target_location) _newtrack_1)) false false))))
    (:then_1
      (bind _newtrack_1_2 (Timeline|Timeline_0 PlayFromStart)
        (:Update
          (Transformation|SetActorLocation (Math|Vector|MakeVector (.x _returnvalue) (+ (.y _target_location) _newtrack_1_2) (.z _returnvalue)) false false))))))

(event EventStopStopAction
  (bind _returnvalue (Transformation|GetActorLocation))
  (bind _returnvalue_2 (Transformation|GetActorLocation))
  (bind _target_location (Variables|Default|GetTarget%20Location))
  (Utilities|FlowControl|Sequence
    (:then_0
      (bind _newtrack_1 (Timeline|Movement Stop)
        (:Update
          (Transformation|SetActorLocation (Math|Vector|MakeVector (.x _returnvalue_2) (.y _returnvalue_2) (+ (.z _target_location) _newtrack_1)) false false))))
    (:then_1
      (bind _newtrack_1_2 (Timeline|Timeline_0 Stop)
        (:Update
          (Transformation|SetActorLocation (Math|Vector|MakeVector (.x _returnvalue) (+ (.y _target_location) _newtrack_1_2) (.z _returnvalue)) false false))))))

(event EventGotHit
  (params (Loosed%20life :type Integer))
  (|CallParentFunction Loosed%20life))

(event EventDie
  (Niagara|SpawnSystematLocation "/Game/Sci-Fi_Starter_VFX_Pack_Niagara/Niagara/Explosion/NS_Explosion_C4_2.NS_Explosion_C4_2" (Transformation|GetActorLocation))
  (bind _outactors (Actor|GetAllActorsOfClass "/Game/Shmup/Blueprints/Player_BP.Player_BP_C"))
  (Default|EndGame (Utilities|Array|Get(acopy) _outactors))
  (|CallParentFunction))

(fn ConstructionScript
  (|CallParentFunction))