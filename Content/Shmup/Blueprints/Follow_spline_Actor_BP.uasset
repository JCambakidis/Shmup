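; Shmup base actor that follows a spline, makes one stop at a target, and destroys itself at the last spline point.
; Tick advances spline distance by MovementSpeed each frame and moves with swept VInterpTo through a Gate.
; Nearing TargetLocation or overlapping TargetActor closes the Gate and calls the empty ActionOnStop hook once.
; An optional TimeBeforeMove delay calls StopStopAction and reopens the Gate.
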(event OnComponentBeginOverlap(Box)
  (params (OverlappedComponent :type Primitive%20Component%20Object%20Reference) (OtherActor :type Actor%20Object%20Reference) (OtherComp :type Primitive%20Component%20Object%20Reference) (OtherBodyIndex :type Integer) (bFromSweep :type Boolean) (SweepResult :type Hit%20Result%20Structure%20%28by%20ref%29))
  (bind _time_before__move (Variables|Default|GetTime%20Before%20%20Move))
  (if (== OtherActor (Variables|Default|GetTarget%20actor))
    (Utilities|FlowControl|Sequence
      (:then_0
        (Utilities|FlowControl|DoOnce false
          (:Completed
            (Variables|Default|SetIn%20place true)
            (CallFunction|ActiononStop)
            (Utilities|FlowControl|Gate false) ; enters at Close
          )))
      (:then_1
        (if (> _time_before__move -1.0)
          (Utilities|FlowControl|Delay _time_before__move)
          (Variables|Default|SetIn%20place false)
          (CallFunction|StopStopAction)
          (Utilities|FlowControl|Gate false) ; enters at Open
        )))))

(event Custom|Action%20On%20Stop)

(event Custom|Stop%20Stop%20Action)

(event EventBeginPlay
  (Utilities|FlowControl|Delay 1.0)
  (Variables|Default|SetCan%20move true))

(event Collision|EventActorBeginOverlap
  (params (OtherActor :type Actor%20Object%20Reference)))

(event EventTick
  (params (DeltaSeconds :type Float%20%28single-precision%29))
  (bind _returnvalue (Transformation|GetActorLocation))
  (bind _spline (Variables|Default|GetSpline))
  (bind _time_before__move (Variables|Default|GetTime%20Before%20%20Move))
  (Utilities|FlowControl|Sequence
    (:then_0
      (Utilities|FlowControl|Gate false :!label _label
        (:Exit
          (Transformation|SetActorLocation (Math|Interpolation|VInterpTo _returnvalue (Spline|GetLocationatDistanceAlongSpline _spline (Variables|Default|GetDistance%20Along%20Spline) "World") DeltaSeconds 1e+01) true false)
          (Variables|Default|SetDistance%20Along%20Spline (+ (Variables|Default|GetDistance%20Along%20Spline) (Variables|Default|GetMovement%20Speed))))))
    (:then_1
      (if (< (Math|Vector|Distance(Vector) _returnvalue (Variables|Default|GetTarget%20Location)) 1e+02)
        (Utilities|FlowControl|Sequence
          (:then_0
            (Utilities|FlowControl|DoOnce false
              (:Completed
                (Variables|Default|SetIn%20place true)
                (CallFunction|ActiononStop)
                (goto _label Close))))
          (:then_1
            (if (> _time_before__move -1.0)
              (Utilities|FlowControl|Delay _time_before__move)
              (Variables|Default|SetIn%20place false)
              (CallFunction|StopStopAction)
              (goto _label Open))))))
    (:then_2
      (if (Math|Vector|Equal(Vector) _returnvalue (Spline|GetLocationatSplinePoint _spline (- (Spline|GetNumberOfSplinePoints _spline) 1) "World") 1e+01)
        (Actor|DestroyActor)))))

(fn ConstructionScript)