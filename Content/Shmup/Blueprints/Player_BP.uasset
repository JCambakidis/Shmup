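; Player pawn for a sprite-based shoot 'em up, handling controls, score and the game start/end cycle.
; Input moves it on the bounded Y/Z plane, with Tick easing it back inside limits and replaying a camera shake.
; Held fire loops through a gate and timer, alternating left and right muzzle sockets.
; PlayGame resets state and starts spawners; hits and death trigger effects, and EndGame shows the results widget and saves the high score.
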(event Custom|Play%20Game
  (Variables|Default|SetGameEnd false)
  (Variables|Default|SetPoints 0)
  (Variables|Default|SetLife (Variables|Default|GetInit%20Life))
  (Variables|Default|SetGame%20Start true)
  (Rendering|SetVisibility (Variables|Default|GetPaperSprite) true true)
  (bind _outactors (Actor|GetAllActorsOfClass "/Game/Shmup/Blueprints/Spawner/BP_Spawner.BP_Spawner_C"))
  (for _array_element _outactors
    (Default|StartMovement _array_element)))

(event Custom|Replace%20Player%20on%20scene
  (bind _returnvalue (Transformation|GetActorLocation))
  (bind _returnvalue_2 (Transformation|GetActorLocation))
  (bind _returnvalue_3 (Transformation|GetActorLocation))
  (bind _returnvalue_4 (Transformation|GetActorLocation))
  (bind _returnvalue_5 (Transformation|GetActorLocation))
  (bind _y_max (Variables|Default|GetY_Max))
  (bind _z_max (Variables|Default|GetZ_Max))
  (bind _z_min (Variables|Default|GetZ_Min))
  (bind _y_min (Variables|Default|GetY_Min))
  (Utilities|FlowControl|Sequence
    (:then_0
      (if (> (.z _returnvalue) _z_max)
        (Transformation|SetActorLocation (Math|Vector|MakeVector (.x _returnvalue_3) (.y _returnvalue_3) (Math|Interpolation|FInterpTo (.z _returnvalue_3) _z_max (Utilities|Time|GetWorldDeltaSeconds) 1e+01)) true false)))
    (:then_1
      (if (< (.z _returnvalue) _z_min)
        (Transformation|SetActorLocation (Math|Vector|MakeVector (.x _returnvalue_4) (.y _returnvalue_4) (Math|Interpolation|FInterpTo (.z _returnvalue_4) _z_min (Utilities|Time|GetWorldDeltaSeconds) 1e+01)) true false)))
    (:then_2
      (if (> (.y _returnvalue) _y_max)
        (Transformation|SetActorLocation (Math|Vector|MakeVector (.x _returnvalue_5) (Math|Interpolation|FInterpTo (.y _returnvalue_5) _y_max (Utilities|Time|GetWorldDeltaSeconds) 1e+01) (.z _returnvalue_5)) true false)))
    (:then_3
      (if (< (.y _returnvalue) _y_min)
        (Transformation|SetActorLocation (Math|Vector|MakeVector (.x _returnvalue_2) (Math|Interpolation|FInterpTo (.y _returnvalue_2) _y_min (Utilities|Time|GetWorldDeltaSeconds) 1e+01) (.z _returnvalue_2)) true false)))))

(event Custom|Add%20Points
  (params (Points%20to%20add :type Integer))
  (Variables|Default|SetPoints (+ (Variables|Default|GetPoints) Points%20to%20add)))

(event Custom|End%20Game
  (bind _returnvalue (Game|GetPlayerController 0))
  (Variables|Default|SetGameEnd true)
  (Variables|Default|SetGame%20Start false)
  (Utilities|FlowControl|Delay 1.0)
  (bind _returnvalue_2 (UserInterface|CreateWidget "/Game/Shmup/Widget/W_EndGame.W_EndGame_C" _returnvalue))
  (Variables|/Game/Shmup/Widget/W_EndGame.W_EndGame_C|SetPoints _returnvalue_2 (Variables|Default|GetPoints))
  (UserInterface|Viewport|AddtoViewport _returnvalue_2 0)
  (Variables|/Script/Engine.PlayerController|SetbShowMouseCursor _returnvalue true)
  (bind _returnvalue_3 (SaveGame|DoesSaveGameExist "save"))
  (if _returnvalue_3
    (bind _returnvalue_4 (SaveGame|LoadGamefromSlot "save"))
    (bind _assave (Utilities|Casting|CastToSave _returnvalue_4))
    (if (< (Variables|/Game/Shmup/Saves/Save.Save_C|GetMax%20Points _assave) (Variables|Default|GetPoints))
      (Variables|/Game/Shmup/Saves/Save.Save_C|SetMax%20Points _assave (Variables|Default|GetPoints))
      (SaveGame|SaveGametoSlot _assave "save"))
    (else
      (bind _returnvalue_5 (SaveGame|CreateSaveGameObject "/Game/Shmup/Saves/Save.Save_C"))
      (if (< (Variables|/Game/Shmup/Saves/Save.Save_C|GetMax%20Points _returnvalue_5) (Variables|Default|GetPoints))
        (Variables|/Game/Shmup/Saves/Save.Save_C|SetMax%20Points _returnvalue_5 (Variables|Default|GetPoints))
        (SaveGame|SaveGametoSlot _returnvalue_5 "save")))))

(event EventBeginPlay)

(event Collision|EventActorBeginOverlap
  (params (OtherActor :type Actor%20Object%20Reference)))

(event EventShoot
  (bind _papersprite (Variables|Default|GetPaperSprite))
  (Utilities|FlowControl|Gate false
    (:Exit
      (if (and (not (Variables|Default|GetGameEnd)) (Variables|Default|GetGame%20Start))
        (Utilities|FlowControl|FlipFlop
          (:A
            (Game|SpawnActorfromClass "/Game/Shmup/Blueprints/Projectiles/Player_simpleshoot_BP.Player_simpleshoot_BP_C" (Math|Transform|MakeTransform (Transformation|GetSocketLocation _papersprite "Shoot_L") "90.000000,90.000000, 0") "Undefined" 0 0))
          (:B
            (Game|SpawnActorfromClass "/Game/Shmup/Blueprints/Projectiles/Player_simpleshoot_BP.Player_simpleshoot_BP_C" (Math|Transform|MakeTransform (Transformation|GetSocketLocation _papersprite "Shoot_R") "90.000000,90.000000, 0") "Undefined" 0 0)))
        (Utilities|Time|SetTimerbyEvent (delegate EventShoot) (Variables|Default|GetShoot%20Speed))))))

(event EventGotHit
  (params (Loosed%20life :type Integer))
  (bind _returnvalue (Transformation|GetActorLocation))
  (if (not (Variables|Default|GetGameEnd))
    (|CallParentFunction Loosed%20life)
    (Niagara|SpawnSystematLocation "/Game/Sci-Fi_Starter_VFX_Pack_Niagara/Niagara/Blood/NS_Blood_Splat_3D_2.NS_Blood_Splat_3D_2" (Math|Vector|MakeVector (+ (.x _returnvalue) -1e+02) (.y _returnvalue) (.z _returnvalue)) "0, 0, 0" "2.000000,2.000000,2.000000")
    (Camera|PlayWorldCameraShake "/Game/Shmup/Blueprints/Camera_shakes/CS_hit.CS_hit_C" (Camera|GetCameraLocation (Game|GetPlayerCameraManager 0)) 0.0 5e+02 1.0 true)))

(event EventDie
  (Utilities|FlowControl|DoOnce false
    (:Completed
      (Rendering|SetVisibility (Variables|Default|GetPaperSprite) false true)
      (Niagara|SpawnSystematLocation "/Game/Sci-Fi_Starter_VFX_Pack_Niagara/Niagara/Explosion/NS_Explosion_C4_2.NS_Explosion_C4_2" (Transformation|GetActorLocation))
      (CallFunction|EndGame))))

(event EventTick
  (params (DeltaSeconds :type Float%20%28single-precision%29))
  (CallFunction|ReplacePlayeronScene)
  (Camera|PlayWorldCameraShake "/Game/Shmup/Blueprints/Camera_shakes/CS_hit1.CS_hit1_C" (Camera|GetCameraLocation (Game|GetPlayerCameraManager 0)) 0.0 5e+02 1.0 true))

(event Input|ActionEvents|InputActionShoot
  (params (Key :type Key%20Structure :default "None"))
  (bind _papersprite (Variables|Default|GetPaperSprite))
  (:Pressed
    (Utilities|FlowControl|Sequence
      (:then_0
        (Utilities|FlowControl|Gate false) ; enters at Open
      )
      (:then_1
        (CallFunction|Shoot))))
  (:Released
    (Utilities|FlowControl|Gate false) ; enters at Close
  ))

(event Input|AxisEvents|InputAxisMoveForward
  (params (AxisValue :type Float%20%28single-precision%29))
  (bind _returnvalue (Transformation|GetActorLocation))
  (bind _returnvalue_2 (* 1e+02 AxisValue))
  (bind _returnvalue_3 (+ (.z _returnvalue) _returnvalue_2))
  (if (Math|Boolean|ANDBoolean (> _returnvalue_3 (Variables|Default|GetZ_Min)) (< _returnvalue_3 (Variables|Default|GetZ_Max)) (not (Variables|Default|GetGameEnd)) (Variables|Default|GetGame%20Start))
    (Pawn|Input|AddMovementInput "0, 0,1.000000" AxisValue false)))

(event Input|AxisEvents|InputAxisMoveRight
  (params (AxisValue :type Float%20%28single-precision%29))
  (bind _returnvalue (Transformation|GetActorLocation))
  (bind _returnvalue_2 (* 5e+02 AxisValue))
  (bind _returnvalue_3 (+ (.y _returnvalue) _returnvalue_2))
  (if (Math|Boolean|ANDBoolean (> _returnvalue_3 (Variables|Default|GetY_Min)) (< _returnvalue_3 (Variables|Default|GetY_Max)) (not (Variables|Default|GetGameEnd)) (Variables|Default|GetGame%20Start))
    (Pawn|Input|AddMovementInput "0.000000,1.000000,0.000000" AxisValue false)))

(fn ConstructionScript)