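; BackGround_BP is a shmup environment actor that produces an endlessly scrolling background from three components: BG, BG1 and BG2.
; Every Tick runs MoveBG on each component, lowering it along relative Z by a fixed step that is not scaled by delta time.
; A component that falls to the lower limit jumps back up to a high Z position, forming the loop.
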(event EventBeginPlay)

(event Collision|EventActorBeginOverlap
  (params (OtherActor :type Actor%20Object%20Reference)))

(event EventTick
  (params (DeltaSeconds :type Float%20%28single-precision%29))
  (Utilities|FlowControl|Sequence
    (:then_0
      (Utilities|MoveBG (Variables|Default|GetBG)))
    (:then_1
      (Utilities|MoveBG (Variables|Default|GetBG2)))
    (:then_2
      (Utilities|MoveBG (Variables|Default|GetBG1)))))

(fn ConstructionScript)