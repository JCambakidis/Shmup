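; Shmup enemy wave spawner that spawns configured actors one by one on a timer at a spline's start.
; Construction script places box components along the spline as formation slots, assigned to enemies in reverse order with movement, life and points settings.
; ProjectileMovement scrolls the spawner, with events to stop and restart it.
; CheckSpawnEnd uses a gate to detect a cleared wave, then restarts all spawners and destroys itself.
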(event Custom|Spawn
  (bind _actors_to_spawn (Variables|Actorconfig|GetActors%20to%20Spawn))
  (bind _newvar_0 (Variables|Default|GetNewVar_0))
  (bind _spawn_index (Variables|Default|GetSpawn%20Index))
  (bind _spawn_index_2 (Variables|Default|GetSpawn%20Index))
  (bind _returnvalue (Utilities|Array|Length _newvar_0))
  (bind _output (Utilities|Array|Get(acopy) _actors_to_spawn _spawn_index))
  (bind (_actor _scale _life _pointstoadd) (Utilities|Struct|BreakFollow_Spline_Actor_Config_S _output))
  (bind _returnvalue_2 (- _returnvalue 1))
  (bind _returnvalue_3 (- _returnvalue_2 _spawn_index_2))
  (bind _output_2 (Utilities|Array|Get(acopy) _newvar_0 _returnvalue_3))
  (if (< _spawn_index (Utilities|Array|Length _actors_to_spawn))
    (bind _returnvalue_4 (Game|SpawnActorfromClass _actor (Math|Transform|MakeTransform (Spline|GetLocationatSplinePoint (Variables|Default|GetSpline) 0 "World") "0,-90.000000,180.000000" _scale) "Undefined" 0 0))
    (Utilities|IsValid _returnvalue_4
      (:Is%20Valid
        (Utilities|Array|Add (Variables|Default|GetSpawned%20Enemy) _returnvalue_4)
        (Variables|/Game/Shmup/Blueprints/Follow_spline_Actor_BP.Follow_spline_Actor_BP_C|SetTime%20Before%20%20Move _returnvalue_4 (Variables|ActorConfig|GetTime%20before%20move))
        (Variables|/Game/Shmup/Blueprints/Follow_spline_Actor_BP.Follow_spline_Actor_BP_C|SetTarget%20actor _returnvalue_4 _output_2)
        (Variables|/Game/Shmup/Blueprints/Follow_spline_Actor_BP.Follow_spline_Actor_BP_C|SetTarget%20Location _returnvalue_4 (Transformation|GetWorldLocation _output_2))
        (Variables|/Game/Shmup/Blueprints/Follow_spline_Actor_BP.Follow_spline_Actor_BP_C|SetMovement%20Speed _returnvalue_4 (Variables|ActorConfig|GetActor%20speed))
        (Variables|/Game/Shmup/Blueprints/Follow_spline_Actor_BP.Follow_spline_Actor_BP_C|SetSpline _returnvalue_4 (Variables|Default|GetSpline))
        (bind _asspace_pawn_bp (Utilities|Casting|CastToSpace_Pawn_BP _returnvalue_4))
        (Variables|/Game/Shmup/Blueprints/Space_Pawn_BP.Space_Pawn_BP_C|SetSpawner%20ref _asspace_pawn_bp self)
        (Variables|/Game/Shmup/Blueprints/Space_Pawn_BP.Space_Pawn_BP_C|SetPoints%20to%20add _asspace_pawn_bp _pointstoadd)
        (Variables|/Game/Shmup/Blueprints/Space_Pawn_BP.Space_Pawn_BP_C|SetLife _asspace_pawn_bp _life)
        (Utilities|Time|SetTimerbyEvent (delegate Custom|Spawn) (Variables|SpawnConfig|GetTime%20between%20two%20enemies))
        (Math|Integer|IncrementInt (Variables|Default|GetSpawn%20Index))))))

(event Custom|Stop%20Movement
  (bind _projectilemovement (Variables|Default|GetProjectileMovement))
  (Variables|/Script/Engine.ProjectileMovementComponent|SetMaxSpeed _projectilemovement 0.0)
  (Variables|/Script/Engine.MovementComponent|SetVelocity _projectilemovement "0, 0, 0"))

(event Custom|Start%20Movement
  (bind _projectilemovement (Variables|Default|GetProjectileMovement))
  (Variables|/Script/Engine.ProjectileMovementComponent|SetMaxSpeed _projectilemovement 1e+03)
  (Variables|/Script/Engine.MovementComponent|SetVelocity _projectilemovement "0, 0,-1000.000000"))

(event Custom|Check%20Spawn%20End
  (Utilities|FlowControl|Delay 0.2)
  (bind _array_element (Utilities|Array|ForEachLoopwithBreak (Variables|Default|GetSpawned%20Enemy) :!label _label)
    (:LoopBody
      (Utilities|IsValid _array_element
        (:Is%20Valid
          (Utilities|FlowControl|Sequence
            (:then_0
              (goto _label_2 Close))
            (:then_1
              (goto _label Break))))
        (:Is%20Not%20Valid
          (goto _label_2 Open))))
    (:Completed
      (Utilities|FlowControl|Gate true :!label _label_2
        (:Exit
          (bind _outactors (Actor|GetAllActorsOfClass "BP_Spawner_C"))
          (for _array_element_2 _outactors
            (CallFunction|StartMovement _array_element_2))
          (Actor|DestroyActor))))))

(event EventBeginPlay)

(fn ConstructionScript
  (bind _spline (Variables|Default|GetSpline))
  (bind _actors_to_spawn (Variables|Actorconfig|GetActors%20to%20Spawn))
  (bind _returnvalue (Utilities|Array|Length _actors_to_spawn))
  (for _index (range 1 _returnvalue)
    (bind _returnvalue_2 (AddComponent|AddBoxComponent true (Math|Transform|MakeTransform (Spline|GetLocationatDistanceAlongSpline _spline (- (* (+ (/ (Spline|GetSplineLength _spline) (Math|Conversions|ToFloat(Integer) _returnvalue)) (Variables|SplineConfig|GetDistance%20between%20actor)) (Math|Conversions|ToFloat(Integer) _index)) (Variables|SplineConfig|GetOffset)) "World"))))
    (Transformation|AttachComponentToComponent _returnvalue_2 (Variables|Default|GetScene) "None" "KeepWorld" "KeepRelative" "KeepRelative" true)
    (Utilities|Array|Add (Variables|Default|GetNewVar_0) _returnvalue_2)))