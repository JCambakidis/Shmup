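; Base pawn for shoot 'em up ships, with life, death and bullet-hell firing helpers.
; GotHit subtracts Life or, once it is negative, calls Die and awards points to the first Player_BP unless that is itself.
; Die notifies a valid spawner before destroying the pawn, while Shoot is an empty event.
; HellShoot spawns an angular fan of projectiles at once; Hell_loop_Shoot staggers one through a delayed-loop macro.
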(event Custom|Got%20Hit
  (params (Loosed%20life :type Integer))
  (if (>= (Variables|Default|GetLife) 0)
    (Variables|Default|SetLife (- (Variables|Default|GetLife) Loosed%20life))
    (else
      (CallFunction|Die)
      (bind _outactors (Actor|GetAllActorsOfClass "/Game/Shmup/Blueprints/Player_BP.Player_BP_C"))
      (if (!= (Utilities|Array|Get(acopy) _outactors) self)
        (Default|AddPoints (Utilities|Array|Get(acopy) _outactors) (Variables|Default|GetPoints%20to%20add))))))

(event Custom|Die
  (bind _spawner_ref (Variables|Default|GetSpawner%20ref))
  (Utilities|IsValid _spawner_ref
    (:Is%20Valid
      (Default|CheckSpawnEnd _spawner_ref))
    (:Is%20Not%20Valid
      _))
  (Actor|DestroyActor))

(event Custom|Shoot)

(event EventBeginPlay
  (Variables|Default|SetInit%20Life (Variables|Default|GetLife)))

(event Collision|EventActorBeginOverlap
  (params (OtherActor :type Actor%20Object%20Reference)))

(event EventTick
  (params (DeltaSeconds :type Float%20%28single-precision%29)))

(fn ConstructionScript)

(fn HellShoot
  (params (ShootClass :type Actor%20Class%20Reference) (Location :type Vector) (Scale :type Vector) (Angle%20Start :type Integer) (Angle%20End :type Integer) (Number%20of%20Projectiles :type Integer))
  (LocalVariables|SetSteps (/ (- Angle%20End Angle%20Start) Number%20of%20Projectiles))
  (LocalVariables|SetAngle Angle%20Start)
  (while (<= (LocalVariables|GetAngle) Angle%20End)
    (Game|SpawnActorfromClass ShootClass (Math|Transform|MakeTransform Location (Math|Rotator|MakeRotator 0.0 (Math|Conversions|ToFloat(Integer) (LocalVariables|GetAngle)) 9e+01) Scale) "Undefined" 0 0)
    (LocalVariables|SetAngle (+ (LocalVariables|GetAngle) (LocalVariables|GetSteps)))))