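; Base projectile Blueprint for the shmup that damages Space_Pawn_BP actors on contact.
; Its Box overlap casts the other actor to Space_Pawn_BP, skips the projectile's Parent, then calls GotHit with Damage and destroys the projectile.
; A delay started on BeginPlay also destroys it after a fixed lifetime, with both paths routed through the DestroyProjectile event.
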(event OnComponentBeginOverlap(Box)
  (params (OverlappedComponent :type Primitive%20Component%20Object%20Reference) (OtherActor :type Actor%20Object%20Reference) (OtherComp :type Primitive%20Component%20Object%20Reference) (OtherBodyIndex :type Integer) (bFromSweep :type Boolean) (SweepResult :type Hit%20Result%20Structure%20%28by%20ref%29))
  (bind _asspace_pawn_bp (Utilities|Casting|CastToSpace_Pawn_BP OtherActor))
  (if (!= OtherActor (Variables|Default|GetParent))
    (Default|GotHit _asspace_pawn_bp (Variables|Default|GetDamage))
    (CallFunction|DestroyProjectile)))

(event Custom|Destroy%20Projectile
  (Actor|DestroyActor))

(event EventBeginPlay
  (Utilities|FlowControl|Delay 5.0)
  (CallFunction|DestroyProjectile))

(event Collision|EventActorBeginOverlap
  (params (OtherActor :type Actor%20Object%20Reference)))

(event EventTick
  (params (DeltaSeconds :type Float%20%28single-precision%29)))

(fn ConstructionScript)