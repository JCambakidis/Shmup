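; Shmup enemy that fires bullet-hell patterns and spawns an explosion effect when it dies.
; Shoot starts shortly after BeginPlay and re-arms on a ShootSpeed timer, firing only while CanShoot and InPlace are true.
; Each volley is a half-circle fan followed by a rapid staggered full ring.
; The Hell_loop_Shoot macro spawns projectiles at evenly stepped pitch angles in either direction, using a delayed for-loop macro.
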(event EventBeginPlay
  (|CallParentFunction)
  (Utilities|FlowControl|Delay 0.2)
  (Variables|Default|SetCan%20Shoot true)
  (CallFunction|Shoot))

(event Collision|EventActorBeginOverlap
  (params (OtherActor :type Actor%20Object%20Reference))
  (|CallParentFunction OtherActor) ; This node is disabled and will not be called.\nDrag off pins to build functionality.
)

(event EventTick
  (params (DeltaSeconds :type Float%20%28single-precision%29))
  (|CallParentFunction DeltaSeconds))

(event EventShoot
  (if (and (Variables|Default|GetCan%20Shoot) (Variables|Default|GetIn%20place))
    (Utilities|HellLoopShoot "/Game/Shmup/Blueprints/Projectiles/Enemy_simpleshoot_BP.Enemy_simpleshoot_BP_C" 0.0 (Transformation|GetActorLocation) "3.000000,3.000000,3.000000" 10 0 -180
      (:Complete
        (Utilities|HellLoopShoot "/Game/Shmup/Blueprints/Projectiles/Enemy_simpleshoot_BP.Enemy_simpleshoot_BP_C" 0.01 (Transformation|GetActorLocation) "3.000000,3.000000,3.000000" 10 0 360
          (:Complete
            _)))))
  (Utilities|Time|SetTimerbyEvent (delegate EventShoot) (Variables|Default|GetShoot%20speed)))

(event EventGotHit
  (params (Loosed%20life :type Integer))
  (|CallParentFunction Loosed%20life))

(event EventDie
  (Niagara|SpawnSystematLocation "/Game/Sci-Fi_Starter_VFX_Pack_Niagara/Niagara/Explosion/NS_Explosion_C4_2.NS_Explosion_C4_2" (Transformation|GetActorLocation))
  (|CallParentFunction))

(fn ConstructionScript
  (|CallParentFunction))